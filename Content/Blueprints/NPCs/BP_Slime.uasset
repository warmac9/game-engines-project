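; BP_Slime is a slime NPC that the player bounces on and can defeat by stomping from above.
; A player hit with a steeply downward normal launches the player upward and, when EnableDeath is set, removes one of three health points.
; At zero it destroys itself, spawns a BP_Health actor flung by a mesh impulse, and sends its GamePhaseTrigger message through the game instance.
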(event `self.ReceiveActorBeginOverlap`
  (params (OtherActor :type "Actor Object Reference")))

(event `self.ReceiveBeginPlay`
  (set `self.HealthPoints` 3))

(event `self.ReceiveHit`
  (params (MyComp :type "PrimitiveComponent Object Reference") (Other :type "Actor Object Reference") (OtherComp :type "PrimitiveComponent Object Reference") (bSelfMoved :type Boolean) (HitLocation :type "Vector Structure") (HitNormal :type "Vector Structure") (NormalImpulse :type "Vector Structure") (Hit :type "HitResult Structure (by ref)"))
  (cast `/Game/Blueprints/Player/BP_PlayerBase` Other)
  (if (< (.z HitNormal) -0.9)
    (`Character.LaunchCharacter` (`GameplayStatics.GetPlayerCharacter` 0) (0.0 0.0 1000.0) false false)
    (if (`self.EnableDeath`)
      (bind _result (`/Engine/EditorBlueprintResources/StandardMacros.DecrementInt` (`self.HealthPoints`))
        (:`  `
          (bind _output_get (set `self.HealthPoints` _result))
          (if (== _output_get 0)
            (`self.K2_DestroyActor`)
            (bind _returnvalue (`|SpawnActorFromClass` "/Game/Blueprints/Collectibles/BP_Health.BP_Health_C" (`self.GetTransform`) "Undefined" "MultiplyWithRoot" null null))
            (`PrimitiveComponent.AddImpulse` (`/Game/Blueprints/Collectibles/BP_Health.StaticMesh` _returnvalue) (460000.0 460000.0 0.0) "None" false)
            (message `/Game/Blueprints/GameState/BPI_TriggerGameState.TriggerGamePhase` (`GameplayStatics.GetGameInstance`) (`self.GamePhaseTrigger`))))))))

(fn `UserConstructionScript`)