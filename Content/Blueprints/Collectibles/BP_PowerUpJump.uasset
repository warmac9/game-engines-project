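; BP_PowerUpJump is a collectible power-up, shown as a mushroom that bobs and spins.
; A timeline drives the mushroom's height and yaw, with a FlipFlop on finish alternating reverse and forward playback for an endless loop.
; Any actor overlap while active clears the Activated flag and hides the actor; the Activate event restores both.
; The file itself applies no jump effect.
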(event `self.ReceiveBeginPlay`
  (set `self.Activated` true)
  (bind (_direction _location) (`Timeline|Timeline` :!label _label)
    (:`Update`
      (`SceneComponent.K2_SetRelativeLocation` (`self.mushroom`) (`KismetMathLibrary.MakeVector` 0.0 0.0 (`KismetMathLibrary.Lerp` 0.0 30.0 _location)) false false)
      (`SceneComponent.K2_SetRelativeRotation` (`self.mushroom`) (`KismetMathLibrary.MakeRotator` 0.0 0.0 (`KismetMathLibrary.Lerp` 0.0 360.0 _location)) false false))
    (:`Finished`
      (`/Engine/EditorBlueprintResources/StandardMacros.FlipFlop`
        (:`A`
          (goto _label :!via `Reverse`))
        (:`B`
          (goto _label))))))

(event `self.ReceiveActorBeginOverlap`
  (params (OtherActor :type "Actor Object Reference"))
  (if (`self.Activated`)
    (set `self.Activated` false)
    (`self.SetActorHiddenInGame` true)))

(event `Activate`
  (set `self.Activated` true)
  (`self.SetActorHiddenInGame` false))

(fn `UserConstructionScript`)