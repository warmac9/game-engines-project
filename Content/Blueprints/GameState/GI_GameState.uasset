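; Game instance that holds the game phase and player health, pushing health changes to the MainHUD progress bar.
; A looping "HearthBeat" timer drains health every second after a start delay and triggers death at zero.
; Death teleports the player to a phase-specific start from BP_ActorReferences, refills health and restarts the timer.
; Dialogs lock movement, pause the drain and pass to the HUD, then restore both on end.
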(event `self.ReceiveInit`
  (set `self.GamePhase` "NewEnumerator0")
  (`self.SetMaxHealthPoints` 100.0)
  (`self.SetHealthPoints` 0.0 true)
  (`self.SetHearthBeat` false)
  (`CharacterMovementComponent.SetMovementMode` (`Character.CharacterMovement` (`GameplayStatics.GetPlayerCharacter` 0)) "MOVE_Walking" 0))

(event `/Game/Blueprints/GameState/BPI_TriggerGameState.Trigger Player Death`
  (params (`Death Type` :type "/Game/Blueprints/Player/E_PlayerDeath Enum" :default "NewEnumerator0"))
  (bind _capsulecomponent (`Character.CapsuleComponent` (`GameplayStatics.GetPlayerCharacter` 0)))
  (`KismetSystemLibrary.PrintString` (`|GetEnumeratorNameAsString` `Death Type`))
  (`PrimitiveComponent.SetPhysicsLinearVelocity` _capsulecomponent (0.0 0.0 0.0) false "None")
  (`PrimitiveComponent.SetPhysicsAngularVelocityInDegrees` _capsulecomponent (0.0 0.0 0.0) false "None")
  (bind _respawnlocation (`self.GetRespawnLocation`))
  (`Actor.K2_SetActorLocationAndRotation` (`GameplayStatics.GetPlayerCharacter` 0) (.location _respawnlocation) (.rotation _respawnlocation) false true)
  (`self.SetHearthBeat` false)
  (`self.SetHealthPoints` 0.0 true)
  (`self.SetHearthBeat` true))

(event `SetHearthBeat`
  (params (Active :type Boolean))
  (if Active
    (bind _returnvalue (`KismetSystemLibrary.K2_SetTimerDelegate` (delegate `HearthBeat`) 1.0 true false 3.0))
    (set `self.HearthBeatTimer` _returnvalue)
    (else
      (`KismetSystemLibrary.K2_ClearAndInvalidateTimerHandle` (`self.HearthBeatTimer`)))))

(event `HearthBeat`
  (`self.SetHealthPoints` -1.0)
  (bind _returnvalue (`GameplayStatics.GetActorOfClass` "/Game/UserInterface/MainHUD.MainHUD_C"))
  (bind _healthpercent (`self.GetHealthPercent`))
  (`/Game/UserInterface/WB_MainHUD.SetHealthProgressBar` (`/Game/UserInterface/MainHUD.MainHUDRef` _returnvalue) _healthpercent)
  (if (<= (`self.HealthPoints`) 0.0)
    (`/Game/Blueprints/GameState/BPI_TriggerGameState.Trigger Player Death` "NewEnumerator1")))

(event `/Game/Blueprints/GameState/BPI_TriggerGameState.Trigger Dialog`
  (params (DialogObject :type "/Game/Blueprints/Dialogs/BP_Dialog Object Reference"))
  (bind _returnvalue (`GameplayStatics.GetPlayerCharacter` 0))
  (`CharacterMovementComponent.DisableMovement` (`Character.CharacterMovement` _returnvalue))
  (`SceneComponent.K2_SetRelativeRotation` :`self` (`Character.Mesh` _returnvalue))
  (`self.SetHearthBeat` false)
  (bind _returnvalue_2 (`GameplayStatics.GetActorOfClass` "/Game/UserInterface/MainHUD.MainHUD_C"))
  (`/Game/UserInterface/WB_MainHUD.TriggerDialog` (`/Game/UserInterface/MainHUD.MainHUDRef` _returnvalue_2) DialogObject))

(event `/Game/Blueprints/GameState/BPI_TriggerGameState.TriggerDialogEnd`
  (params (DialogResult :type "/Game/Blueprints/Dialogs/SDialogResult Structure"))
  (set `/Game/Blueprints/Dialogs/BP_Dialog.TriggeredByPlayer` false (`.DialogObject_11_142B06014F6876D245570C9054628ED6` (break `/Game/Blueprints/Dialogs/SDialogResult` DialogResult)))
  (`CharacterMovementComponent.SetMovementMode` (`Character.CharacterMovement` (`GameplayStatics.GetPlayerCharacter` 0)) "MOVE_Walking" 0)
  (`self.SetHearthBeat` true))

(event `/Game/Blueprints/GameState/BPI_TriggerGameState.TriggerSetPlayerHealth`
  (params (HealthPercent :type "Float (double-precision)"))
  (`self.SetHealthPoints` (* HealthPercent (`self.MaxHealthPoints`)))
  (`self.SetHearthBeat` false)
  (`self.SetHearthBeat` true))

(fn `AddHealthPoints`
  (params (HealthPoints :type "Float (double-precision)"))
  (set `self.HealthPoints` (`KismetMathLibrary.FMax` (`KismetMathLibrary.FMin` (+ HealthPoints (`self.HealthPoints`)) (`self.MaxHealthPoints`)))))

(fn `GetFallToDeathDuration`
  (returns (Duration :type "Float (double-precision)"))
  (return 5.5))

(fn `GetHealthPercent`
  (returns (HealthPercent :type "Float (double-precision)"))
  (return (`KismetMathLibrary.FMin` (`KismetMathLibrary.SafeDivide` (`self.HealthPoints`) (`self.MaxHealthPoints`)) 1.0)))

(fn `GetRespawnLocation`
  (returns (RespawnLocation :type "Transform Structure"))
  (switch `/Game/Blueprints/GameState/E_GamePhase` (`self.GamePhase`)
    (:`NewEnumerator0`
      (bind _returnvalue (`GameplayStatics.GetActorOfClass` "/Game/Blueprints/GameState/BP_ActorReferences.BP_ActorReferences_C"))
      (return (`Actor.GetTransform` (`/Game/Blueprints/GameState/BP_ActorReferences.PlayerStartProlog` _returnvalue))))
    (:`NewEnumerator1`
      (bind _returnvalue_2 (`GameplayStatics.GetActorOfClass` "/Game/Blueprints/GameState/BP_ActorReferences.BP_ActorReferences_C"))
      (return (`Actor.GetTransform` (`/Game/Blueprints/GameState/BP_ActorReferences.PlayerStartProlog2FindingKey` _returnvalue_2))))))

(fn `SetHealthPoints`
  (params (HealthPoints :type "Float (double-precision)") (SetMaxHealth :type Boolean))
  (if SetMaxHealth
    (set `self.HealthPoints` (`self.MaxHealthPoints`))
    (else
      (set `self.HealthPoints` (`KismetMathLibrary.FMax` (`KismetMathLibrary.FMin` (+ HealthPoints (`self.HealthPoints`)) (`self.MaxHealthPoints`))))))
  (bind _returnvalue (`GameplayStatics.GetActorOfClass` "/Game/UserInterface/MainHUD.MainHUD_C"))
  (bind _healthpercent (`self.GetHealthPercent`))
  (`/Game/UserInterface/WB_MainHUD.SetHealthProgressBar` (`/Game/UserInterface/MainHUD.MainHUDRef` _returnvalue) _healthpercent))

(fn `SetMaxHealthPoints`
  (params (HealthPoints :type "Float (double-precision)"))
  (set `self.MaxHealthPoints` HealthPoints)
  (bind _returnvalue (`GameplayStatics.GetActorOfClass` "/Game/UserInterface/MainHUD.MainHUD_C"))
  (bind _healthpercent (`self.GetHealthPercent`))
  (`/Game/UserInterface/WB_MainHUD.SetHealthProgressBar` (`/Game/UserInterface/MainHUD.MainHUDRef` _returnvalue) _healthpercent))