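; Base player character that handles mouse look, jumping and movement, and detects fatal falls.
; Axis inputs move it along yaw-only forward and right vectors, with full sideways input on the ground snapping the mesh to face left or right.
; A looping timer started on BeginPlay tracks continuous falling time.
; Exceeding the Game Instance's fall-to-death duration sends it a player death message.
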(event `InputAxis|Look Up / Down Mouse`
  (params (AxisValue :type "Float (single-precision)"))
  ;[0 0 0] Looking
  (`self.AddControllerPitchInput` (* AxisValue 0.9)))

(event `InputAction|Jump`
  (params (Key :type "Key Structure"))
  ;[0 0 0] Jumping
  (:`Pressed`
    (`self.Jump`))
  (:`Released`
    (`self.StopJumping`)))

(event `InputAxis|Turn Right / Left Mouse`
  (params (AxisValue :type "Float (single-precision)"))
  ;[0 0 0] Looking
  (`self.AddControllerYawInput` (* AxisValue 0.7)))

(event `InputAxis|Move Right / Left`
  (params (AxisValue :type "Float (single-precision)"))
  (bind _mesh (`self.Mesh`))
  ;[0 0 0] Movement
  (`self.AddMovementInput` (`KismetMathLibrary.GetRightVector` (`KismetMathLibrary.MakeRotator` 0.0 0.0 (.yaw (`self.K2_GetActorRotation`)))) AxisValue)
  (if (`NavMovementComponent.IsMovingOnGround` (`self.CharacterMovement`))
    (if (== AxisValue -1.0)
      (`SceneComponent.K2_SetRelativeRotation` _mesh (`KismetMathLibrary.MakeRotator` 0.0 0.0 270.0) false false)
      (elif (== AxisValue 1.0)
        (`SceneComponent.K2_SetRelativeRotation` _mesh (`KismetMathLibrary.MakeRotator` 0.0 0.0 90.0) false false)
        (elif (== (stale `InputAxis|Move Forward / Backward` AxisValue) -1.0)
          (`SceneComponent.K2_SetRelativeRotation` _mesh (`KismetMathLibrary.MakeRotator` 0.0 0.0 180.0) false false)
          (elif (== (stale `InputAxis|Move Forward / Backward` AxisValue) 1.0)
            (`SceneComponent.K2_SetRelativeRotation` _mesh (`KismetMathLibrary.MakeRotator` 0.0) false false)))))))

(event `InputAxis|Move Forward / Backward`
  (params (AxisValue :type "Float (single-precision)"))
  ;[0 0 0] Movement
  (`self.AddMovementInput` (`KismetMathLibrary.GetForwardVector` (`KismetMathLibrary.MakeRotator` 0.0 0.0 (.yaw (`self.K2_GetActorRotation`)))) AxisValue))

(event `self.ReceiveBeginPlay`
  (`self.SetFallDeathCheck` true))

(event `self.ReceiveTick`
  (params (DeltaSeconds :type "Float (single-precision)")))

(event `SetFallDeathCheck`
  (params (Active :type Boolean))
  ;[0 0 0] FallDeathCheck
  (if Active
    (bind _returnvalue (`KismetSystemLibrary.K2_SetTimerDelegate` (delegate `Death Check`) 0.1 true))
    (set `self.DeathCheckTimer` _returnvalue)
    (else
      (`KismetSystemLibrary.K2_ClearAndInvalidateTimerHandle` (`self.DeathCheckTimer`)))))

(event `Death Check`
  ;[0 0 0] FallDeathCheck
  (if (and (`NavMovementComponent.IsFalling` (`self.CharacterMovement`)) (not (`self.WasPlayerFalling`)))
    (set `self.SecondsSinceStartedFalling` (`GameplayStatics.GetTimeSeconds`)))
  (if (not (`NavMovementComponent.IsFalling` (`self.CharacterMovement`)))
    (set `self.SecondsSinceStartedFalling` (`GameplayStatics.GetTimeSeconds`)))
  (set `self.WasPlayerFalling` (`NavMovementComponent.IsFalling` (`self.CharacterMovement`)))
  (if (`NavMovementComponent.IsFalling` (`self.CharacterMovement`))
    (bind _duration (message `/Game/Blueprints/GameState/BPI_GetGameState.GetFallToDeathDuration` (`GameplayStatics.GetGameInstance`)))
    (if (< _duration (- (`GameplayStatics.GetTimeSeconds`) (`self.SecondsSinceStartedFalling`)))
      (set `self.SecondsSinceStartedFalling` (`GameplayStatics.GetTimeSeconds`))
      (message `/Game/Blueprints/GameState/BPI_TriggerGameState.Trigger Player Death` (`GameplayStatics.GetGameInstance`) "NewEnumerator0"))))

(fn `UserConstructionScript`)