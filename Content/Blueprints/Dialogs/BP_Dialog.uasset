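; Dialog actor that triggers a dialog message through the GameInstance when the player stands within its trigger zone.
; A looping timer started on BeginPlay replaces Tick, polling TriggeredByPlayer, grounded movement, min/max 3D distance, height difference and facing angle.
; GetAnglePlayerToNPC derives the player's bearing relative to the actor's yaw using per-quadrant arctangent math.
; The timer keeps running after a trigger unless SetPlayerTriggerCheck(false) clears it.
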(event `self.ReceiveBeginPlay`
  (`self.SetPlayerTriggerCheck` true))

(event `SetPlayerTriggerCheck`
  (params (Active :type Boolean))
  (if Active
    (bind _returnvalue (`KismetSystemLibrary.K2_SetTimerDelegate` (delegate `PlayerTriggerCheck`) 0.1 true))
    (set `self.PlayerTriggerCheckTimer` _returnvalue)
    (else
      (`KismetSystemLibrary.K2_ClearAndInvalidateTimerHandle` (`self.PlayerTriggerCheckTimer`)))))

(event `PlayerTriggerCheck`
  (bind _playertriggeranglethreshold (`self.PlayerTriggerAngleThreshold`))
  (bind _returnvalue (`KismetMathLibrary.Vector_Distance` (`self.K2_GetActorLocation`) (`self.K2_GetActorLocation` (`GameplayStatics.GetPlayerCharacter` 0))))
  (if (`self.TriggeredByPlayer`)
    (if (`NavMovementComponent.IsMovingOnGround` (`Character.CharacterMovement` (`GameplayStatics.GetPlayerCharacter` 0)))
      ;[0 0 0] HorizontalDistance Check
      (if (and (> _returnvalue (`self.PlayerTriggerMinDistance`)) (< _returnvalue (`self.PlayerTriggerMaxDistance`)))
        ;[0 0 0] VerticalDistance Check
        (if (> (`self.PlayerTriggerMaxVertical`) (`KismetMathLibrary.Abs` (.z (- (`self.K2_GetActorLocation`) (`self.K2_GetActorLocation` (`GameplayStatics.GetPlayerCharacter` 0))))))
          ;[0 0 0] AngleCheck
          (bind _degrees (`self.GetAnglePlayerToNPC`))
          (if (or (<= _degrees _playertriggeranglethreshold) (> _degrees (- 360.0 _playertriggeranglethreshold)))
            (message `/Game/Blueprints/GameState/BPI_TriggerGameState.Trigger Dialog` (`GameplayStatics.GetGameInstance`) self)))))))

(fn `GetAnglePlayerToNPC`
  (returns (Degrees :type "Float (double-precision)"))
  (bind _returnvalue (- (`self.K2_GetActorLocation`) (`self.K2_GetActorLocation` (`GameplayStatics.GetPlayerCharacter` 0))))
  (bind _x (.x _returnvalue))
  (bind _y (.y _returnvalue))
  (bind _returnvalue_2 (`KismetMathLibrary.DegAtan` (/ (`KismetMathLibrary.Abs` (.y _returnvalue)) (`KismetMathLibrary.Abs` (.x _returnvalue)))))
  (bind _returnvalue_3 (- (+ (* (+ _returnvalue_2 0.0) (and (not (> _x 0.0)) (not (> _y 0.0)))) (* (+ (- 90.0 _returnvalue_2) 90.0) (and (> _x 0.0) (not (> _y 0.0)))) (* (+ _returnvalue_2 180.0) (and (> _x 0.0) (> _y 0.0))) (* (+ (- 90.0 _returnvalue_2) 270.0) (and (not (> _x 0.0)) (> _y 0.0)))) (.yaw (`self.K2_GetActorRotation`))))
  (if (< _returnvalue_3 0.0)
    (return (+ _returnvalue_3 360.0))
    (else
      (return _returnvalue_3))))

(fn `UserConstructionScript`)