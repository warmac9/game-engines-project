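; BP_PlayerBase is a base player character with mouse look, jumping and movement relative to actor yaw, with strafing at half strength.
; BeginPlay starts a looping timer through SetDeathCheck, which can also stop it.
; Each DeathCheck tracks when falling began and, after a prolonged fall, only prints "dead" without applying an actual death.
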(event `InputAxis|Look Up / Down Mouse`
  (params (AxisValue :type "Float (single-precision)"))
  ;[0 0 0] Looking
  (`self.AddControllerPitchInput` (* AxisValue 0.9)))

(event `InputAction|Jump`
  (params (Key :type "Key Structure"))
  ;[0 0 0] Jumping
  (:`Pressed`
    (`self.Jump`))
  (:`Released`
    (`self.StopJumping`)))

(event `InputAxis|Turn Right / Left Mouse`
  (params (AxisValue :type "Float (single-precision)"))
  ;[0 0 0] Looking
  (`self.AddControllerYawInput` (* AxisValue 0.7)))

(event `InputAxis|Move Right / Left`
  (params (AxisValue :type "Float (single-precision)"))
  ;[0 0 0] Movement
  (`self.AddMovementInput` (`KismetMathLibrary.GetRightVector` (`KismetMathLibrary.MakeRotator` 0.0 0.0 (.yaw (`self.K2_GetActorRotation`)))) (* AxisValue 0.5)))

(event `InputAxis|Move Forward / Backward`
  (params (AxisValue :type "Float (single-precision)"))
  ;[0 0 0] Movement
  (`self.AddMovementInput` (`KismetMathLibrary.GetForwardVector` (`KismetMathLibrary.MakeRotator` 0.0 0.0 (.yaw (`self.K2_GetActorRotation`)))) AxisValue))

(event `self.ReceiveBeginPlay`
  (`self.SetDeathCheck` true))

(event `self.ReceiveTick`
  (params (DeltaSeconds :type "Float (single-precision)")))

(event `SetDeathCheck`
  (params (Active :type Boolean))
  (if Active
    (bind _returnvalue (`KismetSystemLibrary.K2_SetTimerDelegate` (delegate `Death Check`) 0.5 true))
    (set `self.DeathCheckTimer` _returnvalue)
    (else
      (`KismetSystemLibrary.K2_ClearAndInvalidateTimerHandle` (`self.DeathCheckTimer`)))))

(event `Death Check`
  (if (and (`NavMovementComponent.IsFalling` (`self.CharacterMovement`)) (not (`self.WasPlayerFalling`)))
    (set `self.SecondsSinceStartedFalling` (`GameplayStatics.GetTimeSeconds`)))
  (if (not (`NavMovementComponent.IsFalling` (`self.CharacterMovement`)))
    (set `self.SecondsSinceStartedFalling` (`GameplayStatics.GetTimeSeconds`)))
  (set `self.WasPlayerFalling` (`NavMovementComponent.IsFalling` (`self.CharacterMovement`)))
  (if (`NavMovementComponent.IsFalling` (`self.CharacterMovement`))
    (if (> (- (`GameplayStatics.GetTimeSeconds`) (`self.SecondsSinceStartedFalling`)) 5.5)
      (`KismetSystemLibrary.PrintText` "dead"))))

(fn `UserConstructionScript`)