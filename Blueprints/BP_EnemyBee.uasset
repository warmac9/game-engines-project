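; BP_EnemyBee is an enemy bee actor that moves toward points in its PatrolLocations array.
; Each Tick offsets its Capsule along the normalized direction to the current point at MovementSpeed, scaled by delta time and without sweep.
; Within a fixed distance of that point, it sets the index to array length modulo (index + 1), with operands reversed from a usual wraparound, so index 0 never advances.
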(event `self.ReceiveTick`
  (params (DeltaSeconds :type "Float (single-precision)"))
  (set `self.Direction` (- (`|GetArrayItem` (`self.PatrolLocations`) (`self.Location`)) (`self.K2_GetActorLocation`)))
  (`SceneComponent.K2_AddWorldOffset` (`self.Capsule`) (* (* DeltaSeconds (`self.MovementSpeed`)) (`KismetMathLibrary.Normal` (`self.Direction`))) false false)
  (if (< (`KismetMathLibrary.VSize` (`self.Direction`)) 500.0)
    (set `self.Location` (mod (`KismetArrayLibrary.Array_Length` (`self.PatrolLocations`)) (+ (`self.Location`) 1)))))

(fn `UserConstructionScript`)